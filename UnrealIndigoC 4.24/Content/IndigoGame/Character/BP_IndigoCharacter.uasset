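; Player character Blueprint for IndigoGame that handles shoot input, the pause menu and the death screen.
; Shoot input calls Shoot, while Pause input opens the PauseMenu widget.
; BeginPlay binds PlayerDies to the death event, which clears all widgets and shows DeathScreen, ignoring its Time parameter.
; Both menus pause the game, show the mouse cursor and call WidgetReady on the new widget.
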(event `InputAction|Pause`
  (params (Key :type "Key Structure"))
  (bind _returnvalue (`GameplayStatics.GetPlayerController` 0))
  (:`Pressed`
    (bind _returnvalue_2 (`|CreateWidget` "/Game/IndigoGame/UI/PauseMenu.PauseMenu_C" _returnvalue))
    (`UserWidget.AddToViewport` _returnvalue_2 0)
    (`GameplayStatics.SetGamePaused` true)
    (set `PlayerController.bShowMouseCursor` true _returnvalue)
    (`/Game/IndigoGame/UI/PauseMenu.WidgetReady` _returnvalue_2)))

(event `InputAction|Shoot`
  (params (Key :type "Key Structure"))
  (:`Pressed`
    (`self.Shoot` self)))

(event `self.ReceiveBeginPlay`
  (add `self.PlayerDie` (delegate `PlayerDies`)))

(event `PlayerDies` :!signature `self.PlayerDie`
  (params (time :type "Float (double-precision)"))
  (bind _returnvalue (`GameplayStatics.GetPlayerController` 0))
  (`WidgetLayoutLibrary.RemoveAllWidgets`)
  (bind _returnvalue_2 (`|CreateWidget` "/Game/IndigoGame/UI/DeathScreen.DeathScreen_C" _returnvalue))
  (`UserWidget.AddToViewport` _returnvalue_2 0)
  (`GameplayStatics.SetGamePaused` true)
  (set `PlayerController.bShowMouseCursor` true _returnvalue)
  (`/Game/IndigoGame/UI/DeathScreen.WidgetReady` _returnvalue_2))

(fn `UserConstructionScript`)